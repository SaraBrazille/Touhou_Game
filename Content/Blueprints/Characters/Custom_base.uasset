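; Base character with custom physics-driven walking, jumping and flying on a simulated capsule, replacing standard character movement.
; A looping timer applies walk forces and damping or flight physics, with a sphere trace detecting falls.
; Double-pressing jump starts flight, attaching the mesh to the camera for pitch, roll and thrust; any hit restores walking.
; Flight bleeds velocity along camera right and up axes, converting it into forward impulse for gliding.
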(event Collision|EventHit
  (params (MyComp :type Primitive%20Component%20Object%20Reference) (Other :type Actor%20Object%20Reference) (OtherComp :type Primitive%20Component%20Object%20Reference) (bSelfMoved :type Boolean) (HitLocation :type Vector :default "0, 0, 0") (HitNormal :type Vector :default "0, 0, 0") (NormalImpulse :type Vector :default "0, 0, 0") (Hit :type Hit%20Result%20Structure%20%28by%20ref%29))
  (Variables|MovementHandling|SetJumping false)
  (Utilities|IsFlying
    (:Yes
      (CallFunction|StopFly))))

(event Input|ActionEvents|InputActionJump
  (params (Key :type Key%20Structure :default "None"))
  (:Pressed
    (Utilities|IsDoubleJump
      (:Yes
        (Utilities|IsFlying
          (:No
            (CallFunction|StartFly))))
      (:No
        (CallFunction|Jump)))))

(event Input|AxisEvents|InputAxisMoveForward
  (params (AxisValue :type Float%20%28single-precision%29))
  (Variables|MovementHandling|SetPlayerForwardInput AxisValue))

(event Input|AxisEvents|InputAxisMoveRight
  (params (AxisValue :type Float%20%28single-precision%29))
  (Variables|MovementHandling|SetPlayerRightInput AxisValue))

(event Input|AxisEvents|InputAxisLookUp
  (params (AxisValue :type Float%20%28single-precision%29))
  (CallFunction|LookUp AxisValue))

(event Input|AxisEvents|InputAxisTurn
  (params (AxisValue :type Float%20%28single-precision%29))
  (CallFunction|LookRight AxisValue))

(event Input|AxisEvents|InputAxisThrust
  (params (AxisValue :type Float%20%28single-precision%29))
  (Utilities|IsFlying
    (:Yes
      (CallFunction|DoThrust AxisValue))))

(fn ConstructionScript
  (Variables|MovementHandling|SetJumpPressedTime (Math|DateTime|MakeDateTime 1971 0 0))
  (Utilities|Time|SetTimerbyFunctionName 0 "ApplyMovementPhysics" (Variables|Static|GetCustomPhysicsTick) true))

(fn ApplyMovementPhysics
  (CallFunction|FallTest)
  (Utilities|IsFlying
    (:Yes
      (CallFunction|ApplyFlyingPhysics))
    (:No
      (CallFunction|ApplyWalkingPhysics))))

(fn ApplyWalkingPhysics
  (bind _root (Variables|Default|GetRoot))
  (Utilities|IsJumping
    (:Yes
      (Class|PrimitiveComponent|SetLinearDamping (Variables|Default|GetCapsule) 0.01))
    (:No
      (Class|PrimitiveComponent|SetLinearDamping (Variables|Default|GetCapsule) 1e+01)
      (Physics|AddForce (Variables|Default|GetCapsule) (* (Math|Vector|Normalize (+ (* (Math|Vector|GetForwardVector _root) (Variables|MovementHandling|GetPlayerForwardInput)) (* (Math|Vector|GetRightVector _root) (Variables|MovementHandling|GetPlayerRightInput)))) (Variables|MovementHandling|GetMovementSpeed)) "None" true))))

(fn ApplyFlyingPhysics
  (bind _subtractedamount (CallFunction|SubtractPercentfromComponent (Variables|Default|GetCapsule) (Math|Vector|GetRightVector (Variables|Default|GetCamera)) (Variables|Static|GetGravityConversionRate)))
  (LocalVariables|SetForceToAdd (+ _subtractedamount (LocalVariables|GetForceToAdd)))
  (bind _subtractedamount_2 (CallFunction|SubtractPercentfromComponent (Variables|Default|GetCapsule) (Math|Vector|GetUpVector (Variables|Default|GetCamera)) (Variables|Static|GetGravityConversionRate)))
  (LocalVariables|SetForceToAdd (+ _subtractedamount_2 (LocalVariables|GetForceToAdd)))
  (Physics|AddImpulse (Variables|Default|GetCapsule) (* (* (Math|Vector|GetForwardVector (Variables|Default|GetCamera)) (Math|Vector|VectorLength (LocalVariables|GetForceToAdd))) (Variables|Static|GetGravityConversionFactor)) "None" true))

(fn Jump
  (Utilities|IsJumping
    (:No
      (Class|PrimitiveComponent|SetLinearDamping (Variables|Default|GetCapsule) 0.01)
      (Variables|MovementHandling|SetJumping true)
      (Physics|AddImpulse (Variables|Default|GetCapsule) (Math|Vector|MakeVector 0.0 0.0 (Variables|MovementHandling|GetJumpSpeed)) "None" true))))

(fn FallTest
  (bind _capsule (Variables|Default|GetCapsule))
  (bind _returnvalue (Transformation|GetWorldLocation _capsule))
  (bind _capsuleradius (Variables|/Script/Engine.CapsuleComponent|GetCapsuleRadius _capsule))
  (bind _returnvalue_2 (Collision|SphereTraceByChannel _returnvalue (+ _returnvalue (Math|Vector|MakeVector 0.0 0.0 (* (- (Variables|/Script/Engine.CapsuleComponent|GetCapsuleHalfHeight _capsule) _capsuleradius) -1.05))) _capsuleradius "TraceTypeQuery1" false 0 "None"))
  (if (not _returnvalue_2)
    (Variables|MovementHandling|SetJumping true)))

(fn LookUp
  (params (LookUp :type Float%20%28single-precision%29))
  (Utilities|IsFlying
    (:Yes
      _)
    (:No
      _))
  (Transformation|AddLocalRotation (Variables|Default|GetCamera) (Math|Rotator|MakeRotator 0.0 (* LookUp -1.0) 0.0) false false))

(fn LookRight
  (params (LookRight :type Float%20%28single-precision%29))
  (Utilities|IsFlying
    (:Yes
      (Transformation|AddLocalRotation (Variables|Default|GetCamera) (Math|Rotator|MakeRotator LookRight 0.0 0.0) false false))
    (:No
      (Transformation|AddWorldRotation (Variables|Default|GetRoot) (Math|Rotator|MakeRotator 0.0 0.0 LookRight) false false))))

(fn StartFly
  (Variables|MovementHandling|SetMovementMode "Flying")
  (Physics|AddImpulse (Variables|Default|GetCapsule) (Math|Vector|MakeVector 0.0 0.0 (Variables|Static|GetStartFlyForce)) "None" true)
  (Transformation|AttachComponentToComponent (Variables|Default|GetPlayerMesh) (Variables|Default|GetCamera) "None" "KeepRelative" "KeepRelative" "KeepRelative" true))

(fn StopFly
  (Variables|MovementHandling|SetMovementMode "Walking")
  (Transformation|AttachComponentToComponent (Variables|Default|GetPlayerMesh) (Variables|Default|GetRoot) "None" "KeepRelative" "KeepRelative" "KeepRelative" true)
  (Transformation|SetRelativeRotation (Variables|Default|GetCamera) "0, 0, 0" false false))

(fn SubtractPercentfromComponent
  (params (Object :type Primitive%20Component%20Object%20Reference) (DirectionComponent :type Vector) (Percent :type Float%20%28single-precision%29))
  (bind _returnvalue (Transformation|GetComponentVelocity Object))
  (bind _returnvalue_2 (Math|Vector|ProjectVectorontoVector _returnvalue DirectionComponent))
  (bind _returnvalue_3 (* _returnvalue_2 Percent))
  (bind _returnvalue_4 (* _returnvalue_3 -1.0))
  (Physics|AddImpulse Object _returnvalue_4 "None" true)
  (return _returnvalue_4))

(fn DoThrust
  (params (Thrust :type Float%20%28single-precision%29))
  (Physics|AddForce (Variables|Default|GetCapsule) (* (Math|Vector|GetForwardVector (Variables|Default|GetCamera)) (* Thrust (Variables|MovementHandling|GetFlySpeed))) "None" true))